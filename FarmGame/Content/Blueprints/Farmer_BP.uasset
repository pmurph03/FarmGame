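; Farmer Blueprint that drives a rotating 3D cursor for hovering and selecting objects that implement Selectable.
; Each tick it moves an overlap box to the cursor and, while nothing is selected, snaps the cursor onto the first overlapped actor if selectable.
; Left click calls Select on an overlapped object and stores it, or calls Select again on the stored one to release it.
; Per-frame debug strings show overlaps, cursor location and selection.
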(event `self.ReceiveTick`
  (params (DeltaSeconds :type "Float (single-precision)"))
  (bind _overlappingactors (`PrimitiveComponent.GetOverlappingActors` (`self.CursorOverlapBox`) null))
  (`self.Debug Strings` DeltaSeconds)
  (`self.RotateCursorIcon` DeltaSeconds)
  (`self.SetOverlapBoxToCursorPosition`)
  (if (`self.HasSelectedObject`)
    (set `self.IsSelectableHovered` false)
    (elif (> (`KismetArrayLibrary.Array_Length` _overlappingactors) 0)
      (`self.StickCursorToActor` (`KismetArrayLibrary.Array_Get` _overlappingactors)))))

(event `Event Left Click Pressed`
  (`self.Select Overlap Object`))

(fn `Debug Strings`
  (params (A :type "Float (double-precision)"))
  (`|ExecutionSequence`
    (:`then_0`
      (for _array_element (`PrimitiveComponent.GetOverlappingActors` (`self.CursorOverlapBox`) null)
        (`KismetSystemLibrary.PrintString` (`KismetStringLibrary.Concat_StrStr` "Overlapped: " (`KismetStringLibrary.Conv_ObjectToString` _array_element)) true true (struct :`G` 0.66 :`B` 1.0 :`A` 1.0) (`GameplayStatics.GetWorldDeltaSeconds`))))
    (:`then_1`
      (`KismetSystemLibrary.PrintString` (`KismetStringLibrary.Concat_StrStr` "Cursor Location:" (`KismetStringLibrary.Conv_VectorToString` (`SceneComponent.K2_GetComponentLocation` (`self.Cursor`)))) true true (struct :`G` 0.66 :`B` 1.0 :`A` 1.0) (`GameplayStatics.GetWorldDeltaSeconds`)))
    (:`then_2`
      (`KismetSystemLibrary.PrintString` (`KismetStringLibrary.Concat_StrStr` "Selected:" (`KismetSystemLibrary.GetDisplayName` (`KismetSystemLibrary.Conv_InterfaceToObject` (`self.SelectedObject`)))) true true (struct :`G` 0.66 :`B` 1.0 :`A` 1.0) (`GameplayStatics.GetWorldDeltaSeconds`)))
    (:`then_3`
      (return))))

(fn `RotateCursorIcon`
  (params (A :type "Float (double-precision)"))
  (`SceneComponent.K2_AddLocalRotation` (`self.Cursor`) (`KismetMathLibrary.MakeRotator` 0.0 0.0 (* A (`self.CursorRotateSpeed`))) false false)
  (return))

(fn `Select Overlap Object`
  (if (`self.HasSelectedObject`)
    (bind _asselectable (cast `Selectable` (`KismetSystemLibrary.Conv_InterfaceToObject` (`self.SelectedObject`)))
      (:`then`
        (`Selectable.Select` _asselectable)
        (set `self.HasSelectedObject` false)
        (set `self.SelectedObject` null)
        (return))
      (:`CastFailed`
        _))
    (else
      (for _array_element (`PrimitiveComponent.GetOverlappingActors` (`self.CursorOverlapBox`) null)
        (if (not (`self.HasSelectedObject`))
          (bind _asselectable_2 (cast `Selectable` _array_element))
          (`Selectable.Select` _asselectable_2)
          (set `self.SelectedObject` _asselectable_2)
          (set `self.HasSelectedObject` true)
          (return)))))
  (return))

(fn `SetOverlapBoxToCursorPosition`
  (`SceneComponent.K2_SetWorldLocationAndRotation` :`self` (`self.CursorOverlapBox`) :`NewLocation` (`SceneComponent.K2_GetComponentLocation` (`self.Cursor`)))
  (return))

(fn `StickCursorToActor`
  (params (Actor :type "Actor Object Reference"))
  (bind _returnvalue (`GameplayStatics.GetWorldDeltaSeconds`))
  (cast `Selectable` Actor
    (:`then`
      (`KismetSystemLibrary.PrintString` (`KismetStringLibrary.Concat_StrStr` "Sticky/Hovered: " (`KismetStringLibrary.Conv_ObjectToString` Actor)) true true (struct :`G` 0.66 :`B` 1.0 :`A` 1.0) _returnvalue)
      (`SceneComponent.K2_SetWorldLocation` (`self.Cursor`) (`self.K2_GetActorLocation` Actor) false false)
      (set `self.IsSelectableHovered` true)
      (return))
    (:`CastFailed`
      (`KismetSystemLibrary.PrintString` "Stick/Hovered Failed or Nothing Hovered." true true (struct :`G` 0.66 :`B` 1.0 :`A` 1.0) _returnvalue)
      (set `self.IsSelectableHovered` false)
      (return))))

(fn `UserConstructionScript`)