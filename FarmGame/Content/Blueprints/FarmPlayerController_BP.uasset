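; Player controller for the farming game that drives the Farmer_BP pawn and creates its UI widget.
; Axis inputs move the pawn, zoom the spring arm, and rotate the root and pitch-clamped gimbal while right mouse is held or gamepad is active.
; Drift-thresholded axes switch gamepad/mouse mode, which Tick passes to the UI.
; Movement events place the cursor by camera trace or under-mouse hit; left click forwards to the pawn.
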(event `self.ReceiveBeginPlay`
  (bind _asfarmer_bp (cast `/Game/Blueprints/Farmer_BP` (`self.K2_GetPawn`)))
  (set `self.Farmer_BP` _asfarmer_bp)
  (bind _returnvalue (`|CreateWidget` "/Game/Blueprints/FarmPlayer_UI_BP.FarmPlayer_UI_BP_C" self))
  (bind _output_get (set `self.Farmer_UI_BP` _returnvalue))
  (`UserWidget.AddToViewport` _output_get 0))

(event `self.ReceiveTick`
  (params (DeltaSeconds :type "Float (single-precision)"))
  (`KismetSystemLibrary.PrintString` (`KismetStringLibrary.Concat_StrStr` "isGamepad:" (`KismetStringLibrary.Conv_BoolToString` (`self.IsGamePadInput`))) true true (struct :`G` 0.66 :`B` 1.0 :`A` 1.0) (`GameplayStatics.GetWorldDeltaSeconds`))
  (set `/Game/Blueprints/FarmPlayer_UI_BP.IsControllerInput` (`self.IsGamePadInput`) (`self.Farmer_UI_BP`)))

(event `InputAction|RightMouseButton`
  (params (Key :type "Key Structure" :default "AnyKey"))
  ;[1 1 1] Right Mouse Bool
  (:`Pressed`
    (set `self.IsRightMouseButtonDown` true))
  (:`Released`
    (set `self.IsRightMouseButtonDown` false)))

(event `InputAxis|Move Forward`
  (params (AxisValue :type "Float (single-precision)"))
  ;[1 1 1] Movement Controls
  (bind (_returnvalue_x _returnvalue_y) (`KismetMathLibrary.BreakVector` (* (`KismetMathLibrary.Normal` (`KismetMathLibrary.MakeVector` AxisValue (stale `InputAxis|Move Right` AxisValue))) (* (`self.Movement Sensitivity`) (`GameplayStatics.GetWorldDeltaSeconds`)))))
  (`self.K2_AddActorLocalOffset` (`self.Farmer_BP`) (`KismetMathLibrary.MakeVector` _returnvalue_x _returnvalue_y) false false :!label _label))

(event `InputAxis|Move Right`
  (params (AxisValue :type "Float (single-precision)"))
  ;[1 1 1] Movement Controls
  (goto _label))

(event `InputAxis|GamePadDualAxis`
  (params (AxisValue :type "Float (single-precision)"))
  ;[1 1 1] Controller to Mouse Input Bool & Controller Drift Handling
  (if (> (`KismetMathLibrary.Abs` AxisValue) (`self.MinGamepadInputDrift`))
    (set `self.IsGamePadInput` true)))

(event `InputAxis|MouseXY`
  (params (AxisValue :type "Float (single-precision)"))
  ;[1 1 1] Controller to Mouse Input Bool & Controller Drift Handling
  (if (> (`KismetMathLibrary.Abs` AxisValue) (`self.MinGamepadInputDrift`))
    (set `self.IsGamePadInput` false)))

(event `InputAxis|AimElevation`
  (params (AxisValue :type "Float (single-precision)"))
  (bind _returnvalue (* AxisValue (`GameplayStatics.GetWorldDeltaSeconds`) (`self.Camera Sensitivity`)))
  (bind _elevategimbal (`/Game/Blueprints/Farmer_BP.ElevateGimbal` (`self.Farmer_BP`)))
  (bind (_relativerotation_roll _relativerotation_pitch) (`KismetMathLibrary.BreakRotator` (`SceneComponent.RelativeRotation` _elevategimbal)))
  (bind _returnvalue_2 (+ _relativerotation_pitch _returnvalue))
  ;[1 1 1] Y-Camera Rotation
  (if (and (>= (`self.CameraMaxY`) _returnvalue_2) (>= _returnvalue_2 (`self.CameraMinY`)) (or (`self.IsRightMouseButtonDown`) (`self.IsGamePadInput`)))
    (`SceneComponent.K2_AddLocalRotation` _elevategimbal (`KismetMathLibrary.MakeRotator` 0.0 _returnvalue) false false)))

(event `InputAxis|Move Forward`
  (params (AxisValue :type "Float (single-precision)"))
  (bind _farmer_bp (`self.Farmer_BP`))
  (bind (_hitresult _returnvalue) (`self.GetHitResultUnderCursorForObjects` (`|MakeArray` "ObjectTypeQuery5" :!type "EObjectTypeQuery Enum")))
  (bind _camera (`/Game/Blueprints/Farmer_BP.Camera` _farmer_bp))
  ;[1 1 1] Mouse Cursor Decal
  (if (`self.IsGamePadInput`) :!label _label_2
    ;;[1 1 1] If Gamepad Input
    (bind (_outhit _returnvalue_2) (`KismetSystemLibrary.LineTraceSingle` (`SceneComponent.K2_GetComponentLocation` _camera) (* (`SceneComponent.GetForwardVector` _camera) 100000.0) "TraceTypeQuery1"))
    (if _returnvalue_2
      (`SceneComponent.K2_SetWorldLocation` (`/Game/Blueprints/Farmer_BP.Cursor` _farmer_bp) (`.Location` (`GameplayStatics.BreakHitResult` _outhit)) false false))
    (else
      ;;[1 1 1] If Mouse Input
      (if _returnvalue
        (`SceneComponent.K2_SetWorldLocation` (`/Game/Blueprints/Farmer_BP.Cursor` _farmer_bp) (`.Location` (`GameplayStatics.BreakHitResult` _hitresult)) false false)))))

(event `InputAction|LeftMouseButton`
  (params (Key :type "Key Structure" :default "AnyKey"))
  ;[1 1 1] LeftClick
  (:`Pressed`
    (`/Game/Blueprints/Farmer_BP.Event Left Click Pressed` (`self.Farmer_BP`))))

(event `InputAxis|Move Right`
  (params (AxisValue :type "Float (single-precision)"))
  ;[1 1 1] Mouse Cursor Decal
  (goto _label_2))

(event `InputAxis|Zoom`
  (params (AxisValue :type "Float (single-precision)"))
  (bind _springarm (`/Game/Blueprints/Farmer_BP.SpringArm` (`self.Farmer_BP`)))
  ;[1 1 1] Zoom: TODO Smooth zoom.
  (set `SpringArmComponent.TargetArmLength` (- (`SpringArmComponent.TargetArmLength` _springarm) (* AxisValue (`self.Zoom Sensitivity`))) _springarm))

(event `InputAxis|AimAzimuth`
  (params (AxisValue :type "Float (single-precision)"))
  ;[1 1 1] Z-Camera Rotation
  (if (or (`self.IsRightMouseButtonDown`) (`self.IsGamePadInput`))
    (`SceneComponent.K2_AddLocalRotation` (`/Game/Blueprints/Farmer_BP.FarmerRoot` (`self.Farmer_BP`)) (`KismetMathLibrary.MakeRotator` 0.0 0.0 (* AxisValue (`GameplayStatics.GetWorldDeltaSeconds`) (`self.Camera Sensitivity`))) false false)))

(fn `UserConstructionScript`)