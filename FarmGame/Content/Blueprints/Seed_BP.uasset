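; Seed actor that the player carries with the farmer's cursor and plants by releasing it, turning it into a plant.
; While held, Tick snaps the seed mesh to the cursor plus an offset and stops the planting timeline.
; Releasing through Hold flags Tick to play that timeline, which cumulatively moves and spins the mesh by its ZPos track.
; When the timeline finishes, the seed spawns PlantBlueprint at the mesh and destroys itself.
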(event `self.ReceiveBeginPlay`
  (bind _asfarmer_bp (cast `/Game/Blueprints/Farmer_BP` (`GameplayStatics.GetPlayerPawn` 0)))
  (set `self.Farmer` _asfarmer_bp))

(event `self.ReceiveTick`
  (params (DeltaSeconds :type "Float (single-precision)"))
  (bind _seedmesh (`self.SeedMesh`))
  (bind _seedmesh_2 (`self.SeedMesh`))
  (bind (_returnvalue_x _returnvalue_y) (`KismetMathLibrary.BreakVector` (`SceneComponent.K2_GetComponentLocation` _seedmesh_2)))
  (bind (_returnvalue_x_2 _returnvalue_y_2 _returnvalue_z) (`KismetMathLibrary.BreakVector` (`SceneComponent.K2_GetComponentLocation` _seedmesh)))
  (if (`self.bIsHeld`)
    (`self.SetWorldPositionToCursor`)
    (bind (_direction _zpos) (`Timeline|Anim_PlantSeed` :!via `Stop` :!label _label)
      (:`Update`
        (bind _returnvalue (+ (`KismetMathLibrary.MakeVector` _returnvalue_x_2 _returnvalue_y_2 _returnvalue_z) (`KismetMathLibrary.MakeVector` 0.0 0.0 _zpos)))
        (`SceneComponent.K2_SetWorldLocation` _seedmesh _returnvalue false false)
        (`KismetSystemLibrary.PrintString` (`KismetStringLibrary.Concat_StrStr` "seed Pos:" (`KismetStringLibrary.Conv_VectorToString` _returnvalue)) true true (struct :`G` 0.66 :`B` 1.0 :`A` 1.0) (`GameplayStatics.GetWorldDeltaSeconds`))
        (`SceneComponent.K2_AddWorldRotation` _seedmesh (`KismetMathLibrary.MakeRotator` _zpos _zpos _zpos) false false))
      (:`Finished`
        (`SceneComponent.K2_SetWorldLocationAndRotation` :`self` _seedmesh_2 :`NewLocation` (`KismetMathLibrary.MakeVector` _returnvalue_x _returnvalue_y))
        (`self.SpawnPlant`)
        (`self.K2_DestroyActor`)))
    (elif (`self.PlayPlantSeed`)
      (set `self.PlayPlantSeed` false)
      (goto _label :!via `PlayFromStart`))))

(fn `GetIsHeld`
  (returns (ReturnValue :type Boolean))
  (return (`self.bIsHeld`)))

(fn `Hold`
  (returns (ReturnValue :type Boolean))
  (if (`self.bIsHeld`)
    (set `self.bIsHeld` false)
    (set `self.PlayPlantSeed` true)
    (else
      (set `self.bIsHeld` true)))
  (return false))

(fn `Select`
  (returns (ReturnValue :type Boolean))
  ;[1 0 0.02836] TODO: Display UI when just selected
  (if (`self.bIsSelected`)
    (set `self.bIsSelected` false)
    (return false)
    (else
      (set `self.bIsSelected` true)
      (return false))))

(fn `SetIsHeld`
  (params (IsHeld :type Boolean))
  (returns (ReturnValue :type Boolean))
  (set `self.bIsHeld` IsHeld)
  (return false))

(fn `SetWorldPositionToCursor`
  (`SceneComponent.K2_SetWorldLocation` (`self.SeedMesh`) (+ (`SceneComponent.K2_GetComponentLocation` (`/Game/Blueprints/Farmer_BP.Cursor` (`self.Farmer`))) (`self.SelectedPositionOffset`)) false false))

(fn `SpawnPlant`
  (bind _seedmesh (`self.SeedMesh`))
  (`|SpawnActorFromClass` (`self.PlantBlueprint`) (`KismetMathLibrary.MakeTransform` (`SceneComponent.K2_GetComponentLocation` _seedmesh) (`SceneComponent.K2_GetComponentRotation` _seedmesh)) "Undefined" "OverrideRootScale"))

(fn `UserConstructionScript`)