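; Flower plant Blueprint that tracks its flowerheads and grows extra stems when fertilized.
; BeginPlay registers the child-actor flowerhead and binds its done-flowering dispatcher to set the finished flag.
; Each fertilizer addition below the maximum spawns a FlowerStem at a socket named by the current count and registers its flowerhead.
; Selecting the plant after flowering fires the release-flowerheads dispatcher; Select always returns false.
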(event `self.ReceiveBeginPlay`
  (`parent.ReceiveBeginPlay`)
  (bind _asflowerhead_bp (cast `/Game/Blueprints/FlowerHead_BP` (`ChildActorComponent.ChildActor` (`self.Flowerhead_BP`))))
  (`KismetArrayLibrary.Array_Add` (`self.Flowerheads`) _asflowerhead_bp)
  (add `/Game/Blueprints/FlowerHead_BP.DoneFlowering Notify Event Dispatcher` _asflowerhead_bp (delegate `Event Done Flowering`)))

(event `self.ReceiveTick`
  (params (DeltaSeconds :type "Float (single-precision)"))
  ;[1 0 0] TODO: Remove tick after growing?
  (`parent.ReceiveTick` DeltaSeconds))

(event `Event Done Flowering`
  (set `self.bFinishedFlowering` true))

(event `self.Event Add Fertilizer`
  (if (< (`self.FertilizeCurrent`) (`self.FertilizeMax`))
    (`parent.Event Add Fertilizer`)
    (bind _returnvalue (`|SpawnActorFromClass` (`self.FlowerStem`) (`SceneComponent.GetSocketTransform` (`self.PlantMesh`) (`KismetStringLibrary.Conv_StringToName` (`KismetStringLibrary.Concat_StrStr` "FertilizePosition_0" (`KismetStringLibrary.Conv_IntToString` (`self.FertilizeCurrent`)))) "RTS_World") "Undefined" "OverrideRootScale" self))
    (`KismetArrayLibrary.Array_Add` (`self.FlowerStems`) _returnvalue)
    (bind (_cast_success _flowerhead_bp) (`/Game/Blueprints/FlowerStem_BP.Get Flowerhead` _returnvalue))
    (if _cast_success
      (`KismetArrayLibrary.Array_Add` (`self.Flowerheads`) _flowerhead_bp))))

(fn `Select`
  (returns (ReturnValue :type Boolean))
  (if (`self.bFinishedFlowering`)
    (`self.Event Release Flowerheads Dispatcher`)
    (return false)
    (else
      (return false))))

(fn `UserConstructionScript`
  (`parent.UserConstructionScript`))