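; Flowerhead actor, parented to a Flower_BP or FlowerStem_BP, that blooms once its owner finishes growing.
; It binds to the parent's dispatchers on BeginPlay and holds the skeletal mesh animation paused until growth completes.
; A done-flowering notify swaps the animated mesh for a static mesh at the same relative transform and prints the sell price.
; Releasing the flowerhead only prints a message, with regrowth left as a TODO.
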(event `self.ReceiveBeginPlay`
  (bind _returnvalue (`self.GetParentActor`))
  (bind _plantowner (`self.PlantOwner`))
  (bind _sk_flowerhead (`self.SK_Flowerhead`))
  (add `self.DoneFlowering Notify Event Dispatcher` (delegate `Event Finished Flowering`))
  (`SceneComponent.SetVisibility` (`self.SM_Flowerhead`) false false)
  (set `SkeletalMeshComponent.bPauseAnims` true _sk_flowerhead)
  (`SceneComponent.SetVisibility` _sk_flowerhead true false)
  (bind _asflower_bp (cast `/Game/Blueprints/Flower_BP` _returnvalue)
    (:`then`
      (set `self.PlantOwner` _asflower_bp)
      (add `/Game/Blueprints/Plant_BP.Finish Growing Dispatcher` _plantowner (delegate `Event Play Flowerhead Anim`))
      (add `/Game/Blueprints/Flower_BP.Event Release Flowerheads Dispatcher` _plantowner (delegate `Event Release Flowerheads`)))
    (:`CastFailed`
      (`KismetSystemLibrary.PrintString` "fail flower")
      (bind _asflower_stem_bp (cast `/Game/Blueprints/FlowerStem_BP` _returnvalue))
      (bind _output_get (set `self.StemOwner` _asflower_stem_bp))
      (add `/Game/Blueprints/FlowerStem_BP.Event Finish Growing Dispatcher ` _output_get (delegate `Event Play Flowerhead Anim`))
      (add `/Game/Blueprints/FlowerStem_BP.Event Release Flowerhead Dispatcher` _output_get (delegate `Event Release Flowerheads`)))))

(event `Event Play Flowerhead Anim`
  (set `SkeletalMeshComponent.bPauseAnims` false (`self.SK_Flowerhead`)))

(event `Event Release Flowerheads`
  ;[1 1 1] TODO: regrow flowerhead
  (`KismetSystemLibrary.PrintString` "Release flowerhead"))

(event `Event Finished Flowering`
  (bind _sm_flowerhead (`self.SM_Flowerhead`))
  (`SceneComponent.SetVisibility` (`self.SK_Flowerhead`) false false)
  (`SceneComponent.SetVisibility` _sm_flowerhead true false)
  (`SceneComponent.K2_SetRelativeTransform` _sm_flowerhead (`SceneComponent.GetRelativeTransform` (`self.SK_Flowerhead`)) false false)
  (bind _returnvalue (`PriceComponent.GetPlayerSellPrice` (`self.Price`)))
  (`KismetSystemLibrary.PrintString` (`KismetStringLibrary.Conv_DoubleToString` _returnvalue)))

(fn `UserConstructionScript`)