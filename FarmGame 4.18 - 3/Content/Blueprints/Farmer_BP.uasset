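; Farmer_BP is the player's farming cursor for selecting, tending and holding objects.
; Each tick it spins the cursor, moves an overlap box to it, prints debug strings and, when empty-handed, snaps to hovered Selectable or Holdable actors and flags plant UI.
; Left click switches on FarmerTool to toggle selection (also calling a currency update), fertilize plants, water plants or toggle holding.
; TODOs note watering needs held input and plan context-based tools.
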(event `self.ReceiveTick`
  (params (DeltaSeconds :type "Float (single-precision)"))
  (bind _overlappingactors (`PrimitiveComponent.GetOverlappingActors` (`self.CursorOverlapBox`) null))
  (`self.Debug Strings` DeltaSeconds)
  (`self.RotateCursorIcon` DeltaSeconds)
  (`self.SetOverlapBoxToCursorPosition`)
  (if (`self.bHasHeldObject`)
    _
    (elif (> (`KismetArrayLibrary.Array_Length` _overlappingactors) 0)
      (`self.StickCursorToActor` (`|GetArrayItem` _overlappingactors))
      (for _array_element _overlappingactors
        (bind _asplant_bp (cast `/Game/Blueprints/Plant_BP` _array_element))
        (set `/Game/Blueprints/Plant_BP.bDisplayUIToggle` true _asplant_bp)))))

(event `Event Left Click Pressed`
  (bind _overlappingactors (`PrimitiveComponent.GetOverlappingActors` (`self.CursorOverlapBox`) "/Game/Blueprints/Plant_BP.Plant_BP_C"))
  (bind _overlappingactors_2 (`PrimitiveComponent.GetOverlappingActors` (`self.CursorOverlapBox`) "/Game/Blueprints/Plant_BP.Plant_BP_C"))
  ;[1 0 0] TODO: Context Select/Hold (As opposed to seperate tools)
  (switch `int` (`self.Farmer_Tool`)
    (:`0`
      (`self.Select Overlap Object`)
      (`self.Update Currency Dispatcher` 100))
    (:`1`
      (if (> (`KismetArrayLibrary.Array_Length` _overlappingactors) 0)
        (for _array_element _overlappingactors
          (bind _asplant_bp (cast `/Game/Blueprints/Plant_BP` _array_element))
          (`/Game/Blueprints/Plant_BP.Event Add Fertilizer` _asplant_bp))))
    (:`2`
      ;[1 0 0.01661] TODO: Doesn't work cause has to be held
      (if (> (`KismetArrayLibrary.Array_Length` _overlappingactors_2) 0)
        (for _array_element_2 _overlappingactors_2
          (bind _asplant_bp_2 (cast `/Game/Blueprints/Plant_BP` _array_element_2))
          ;[1 0 0] TODO: Upgradeable water per second
          (`/Game/Blueprints/Plant_BP.Event Water Plant` _asplant_bp_2 100.0))))
    (:`3`
      (`self.HoldHoldableObject`))))

(fn `Debug Strings`
  (params (A :type "Float (double-precision)"))
  (`|ExecutionSequence`
    (:`then_0`
      (for _array_element (`PrimitiveComponent.GetOverlappingActors` (`self.CursorOverlapBox`) null)
        (`KismetSystemLibrary.PrintString` (`KismetStringLibrary.Concat_StrStr` "Overlapped: " (`KismetStringLibrary.Conv_ObjectToString` _array_element)) true true (struct :`G` 0.66 :`B` 1.0 :`A` 1.0) (`GameplayStatics.GetWorldDeltaSeconds`))))
    (:`then_1`
      (`KismetSystemLibrary.PrintString` (`KismetStringLibrary.Concat_StrStr` "Cursor Location:" (`KismetStringLibrary.Conv_VectorToString` (`SceneComponent.K2_GetComponentLocation` (`self.Cursor`)))) true true (struct :`G` 0.66 :`B` 1.0 :`A` 1.0) (`GameplayStatics.GetWorldDeltaSeconds`)))
    (:`then_2`
      (`KismetSystemLibrary.PrintString` (`KismetStringLibrary.Concat_StrStr` "Selected:" (`KismetSystemLibrary.GetDisplayName` (`KismetSystemLibrary.Conv_InterfaceToObject` (`self.SelectedObject`)))) true true (struct :`G` 0.66 :`B` 1.0 :`A` 1.0) (`GameplayStatics.GetWorldDeltaSeconds`)))
    (:`then_3`
      (return))))

(fn `HoldHoldableObject`
  (if (`self.bHasHeldObject`)
    (`Holdable.Hold` (`self.HeldObject`))
    (set `self.bHasHeldObject` false)
    (set `self.HeldObject` null)
    (return)
    (else
      (for _array_element (`PrimitiveComponent.GetOverlappingActors` (`self.CursorOverlapBox`) null)
        (if (not (`self.bHasHeldObject`))
          (bind _asholdable (cast `Holdable` _array_element))
          (`Holdable.Hold` _asholdable)
          (set `self.HeldObject` _asholdable)
          (set `self.bHasHeldObject` true)
          (return)))
      (return))))

(fn `RotateCursorIcon`
  (params (A :type "Float (double-precision)"))
  (`SceneComponent.K2_AddLocalRotation` (`self.Cursor`) (`KismetMathLibrary.MakeRotator` 0.0 0.0 (* A (`self.CursorRotateSpeed`))) false false)
  (return))

(fn `Select Overlap Object`
  (if (`self.HasSelectedObject`)
    (bind _asselectable (cast `Selectable` (`KismetSystemLibrary.Conv_InterfaceToObject` (`self.SelectedObject`)))
      (:`then`
        (`Selectable.Select` _asselectable)
        (set `self.HasSelectedObject` false)
        (set `self.SelectedObject` null)
        (return))
      (:`CastFailed`
        _))
    (else
      (for _array_element (`PrimitiveComponent.GetOverlappingActors` (`self.CursorOverlapBox`) null)
        (if (not (`self.HasSelectedObject`))
          (bind _asselectable_2 (cast `Selectable` _array_element))
          (`Selectable.Select` _asselectable_2)
          (set `self.SelectedObject` _asselectable_2)
          (set `self.HasSelectedObject` true)
          (return)))))
  (return))

(fn `SetOverlapBoxToCursorPosition`
  (`SceneComponent.K2_SetWorldLocationAndRotation` :`self` (`self.CursorOverlapBox`) :`NewLocation` (`SceneComponent.K2_GetComponentLocation` (`self.Cursor`)))
  (return))

(fn `StickCursorToActor`
  (params (Actor :type "Actor Object Reference"))
  (bind _returnvalue (`GameplayStatics.GetWorldDeltaSeconds`))
  (cast `Selectable` Actor
    (:`then`
      _)
    (:`CastFailed`
      (cast `Holdable` Actor
        (:`then`
          _)
        (:`CastFailed`
          (`KismetSystemLibrary.PrintString` "Stick/Hovered Failed or Nothing Hovered." true true (struct :`G` 0.66 :`B` 1.0 :`A` 1.0) _returnvalue)
          (return)))))
  (`KismetSystemLibrary.PrintString` (`KismetStringLibrary.Concat_StrStr` "Sticky/Hovered: " (`KismetStringLibrary.Conv_ObjectToString` Actor)) true true (struct :`G` 0.66 :`B` 1.0 :`A` 1.0) _returnvalue)
  (`SceneComponent.K2_SetWorldLocation` (`self.Cursor`) (`self.K2_GetActorLocation` Actor) false false)
  (return))

(fn `UserConstructionScript`)