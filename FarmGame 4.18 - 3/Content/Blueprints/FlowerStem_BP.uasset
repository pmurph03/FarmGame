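; FlowerStem_BP is a stem actor owned by a Flower_BP that grows with the plant and hosts a FlowerHead_BP child actor.
; On BeginPlay it caches both references, binds to the parent's dispatchers and records the plant mesh's starting scale.
; Grow events set the stem's uniform world scale to the plant's scale minus that recorded value.
; Finish-growing and release-flowerhead events are relayed through the stem's own dispatchers with debug prints.
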(event `self.ReceiveBeginPlay`
  (bind _parentflower (`self.ParentFlower`))
  (bind _asflower_head_bp (cast `/Game/Blueprints/FlowerHead_BP` (`ChildActorComponent.ChildActor` (`self.FlowerHead_BP`))))
  (set `self.Flower Head` _asflower_head_bp)
  (bind _asflower_bp (cast `/Game/Blueprints/Flower_BP` (`self.GetOwner`)))
  (bind _output_get (set `self.ParentFlower` _asflower_bp))
  (add `/Game/Blueprints/Plant_BP.Grow Plant Dispatcher` _asflower_bp (delegate `Event Grow Stem`))
  (`SceneComponent.SetWorldScale3D` (`self.Stem`) (`KismetMathLibrary.Conv_DoubleToVector` (`Plant.GrowthStartScale` _output_get)))
  (bind _returnvalue_x (`KismetMathLibrary.BreakVector` (`SceneComponent.K2_GetComponentScale` (`/Game/Blueprints/Plant_BP.PlantMesh` _output_get))))
  (set `self.ScaleDifferenceToParent` _returnvalue_x)
  (add `/Game/Blueprints/Plant_BP.Finish Growing Dispatcher` _parentflower (delegate `Event Finish Growing`))
  (add `/Game/Blueprints/Flower_BP.Event Release Flower Heads Dispatcher` _parentflower (delegate `Event Release Flowerheads`)))

(event `Event Finish Growing`
  (`self.Event Finish Growing Dispatcher `)
  (`KismetSystemLibrary.PrintString` "Stem Finished Growing"))

(event `Event Release Flowerheads`
  (`self.Event Release Flowerhead Dispatcher`)
  (`KismetSystemLibrary.PrintString` "Stem Release FlowerHead"))

(event `Event Grow Stem`
  (bind _parentflower (`self.ParentFlower`))
  (bind _returnvalue_x (`KismetMathLibrary.BreakVector` (`SceneComponent.K2_GetComponentScale` (`/Game/Blueprints/Plant_BP.PlantMesh` _parentflower))))
  (if (`KismetSystemLibrary.IsValid` _parentflower)
    (`SceneComponent.SetWorldScale3D` (`self.Stem`) (`KismetMathLibrary.Conv_DoubleToVector` (- _returnvalue_x (`self.ScaleDifferenceToParent`))))))

(fn `Get Flowerhead`)

(fn `UserConstructionScript`)