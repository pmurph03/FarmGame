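; Vegetable actor, a child of a growable plant base, that pops loose when it finishes growing.
; On BeginPlay it binds to the finish-growing dispatcher, which turns on mesh physics and launches the plant upward with a random spin.
; A TODO notes that popping out above ground is not yet ensured.
; The Select override calls the parent, prints a debug string and returns false.
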(event `self.ReceiveBeginPlay`
  (`parent.ReceiveBeginPlay`)
  (add `self.Finish Growing Dispatcher` (delegate `FinishGrowing`)))

(event `FinishGrowing`
  (bind _plantmesh (`self.PlantMesh`))
  ;[1 1 1] TODO: Make sure it pops out above ground..
  (`PrimitiveComponent.SetSimulatePhysics` _plantmesh true)
  (`PrimitiveComponent.AddImpulse` _plantmesh (* (`SceneComponent.GetUpVector` _plantmesh) 500.0) "None" true)
  (`PrimitiveComponent.AddAngularImpulse` _plantmesh (`KismetMathLibrary.MakeVector` (`KismetMathLibrary.RandomFloatInRange` -10.0 10.0) (`KismetMathLibrary.RandomFloatInRange` -10.0 10.0) (`KismetMathLibrary.RandomFloatInRange` -10.0 10.0)) "None" true))

(fn `Select`
  (returns (ReturnValue :type Boolean))
  (`parent.Select`)
  (`KismetSystemLibrary.PrintString` "VeggieSelected")
  (return false))

(fn `UserConstructionScript`
  (`parent.UserConstructionScript`))