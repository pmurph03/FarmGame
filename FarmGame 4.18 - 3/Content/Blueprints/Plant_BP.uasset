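; Growable plant actor that scales its mesh over time, driven by watering and fertilizer.
; Each tick drains water and advances growth fastest at water level 50, firing dispatchers and stopping tick when grown.
; Fertilizer, capped at a maximum, raises final scale and recomputes growth time from current scale.
; A camera-facing widget shows plant stats on ticks where its display flag is set, then clears the flag.
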(event `self.ReceiveBeginPlay`
  (set `self.bIsGrowing` true)
  (`KismetSystemLibrary.PrintString` "Plant: BeginPlay" true true (struct :`G` 0.66 :`B` 1.0 :`A` 1.0) 2.0)
  (`SceneComponent.SetWorldScale3D` (`self.PlantMesh`) (`KismetMathLibrary.Conv_DoubleToVector` (`self.GrowthStartScale`)))
  (add `self.Add Fertilizer Dispatcher` (delegate `Event Add Fertilizer`)))

(event `Event Add Fertilizer`
  (if (`self.bIsGrowing`)
    (if (<= (+ (`self.FertilizeCurrent`) 1) (`self.FertilizeMax`))
      (set `self.FertilizeCurrent` (+ (`self.FertilizeCurrent`) 1))
      (set `self.bJustFertilized` true))))

(event `self.ReceiveTick`
  (params (DeltaSeconds :type "Float (single-precision)"))
  (bind _bdisplayuitoggle (`self.bDisplayUIToggle`))
  (`SceneComponent.SetVisibility` (`self.UI Component`) _bdisplayuitoggle false)
  (if _bdisplayuitoggle
    (`self.UpdateUI`)
    (set `self.bDisplayUIToggle` false))
  (if (`self.bIsGrowing`)
    (`self.GrowPlant`)
    (`self.Grow Plant Dispatcher`)
    (else
      (`self.SetActorTickEnabled` false)
      (`KismetSystemLibrary.PrintString` "Plant: Done Growing, Stopping Tick"))))

(event `Event Water Plant`
  (params (WaterIncreasePerSecond :type "Float (double-precision)"))
  (set `self.WaterCurrentLevel` (`KismetMathLibrary.FClamp` (+ (* WaterIncreasePerSecond (`GameplayStatics.GetWorldDeltaSeconds`)) (`self.WaterCurrentLevel`)) 0.0 (`self.WaterLevelMax`))))

(fn `DecreaseWaterLevel`
  (set `self.WaterCurrentLevel` (`KismetMathLibrary.FClamp` (- (`self.WaterCurrentLevel`) (* (`self.WaterDecreasePerSecond`) (`GameplayStatics.GetWorldDeltaSeconds`))) 0.0 (`self.WaterLevelMax`)))
  (return))

(fn `GrowPlant`
  (bind _returnvalue_x (`KismetMathLibrary.BreakVector` (`SceneComponent.K2_GetComponentScale` (`self.PlantMesh`))))
  (bind _returnvalue (+ (`self.GrowthTimeCurrent`) (* (`GameplayStatics.GetWorldDeltaSeconds`) (- 1.0 (`KismetMathLibrary.Abs` (- (/ (`self.WaterCurrentLevel`) 50.0) 1.0))))))
  (if (`self.bIsGrowing`)
    (if (`self.bJustFertilized`)
      ;[1 0.5426 0.9995] Update Growth Time if just fertilized
      (set `self.bJustFertilized` false)
      (set `self.GrowthTimeCurrent` (* (/ _returnvalue_x (+ (* (`self.FertilizeCurrent`) (`self.FertilizeGrowthMultiplier`)) (`self.BaseFinalScale`))) (`self.GrowthTimeMax`))))
    (`self.DecreaseWaterLevel`)
    (if (<= _returnvalue (`self.GrowthTimeMax`))
      (set `self.GrowthTimeCurrent` _returnvalue)
      (else
        (set `self.GrowthTimeCurrent` (`self.GrowthTimeMax`))
        (set `self.bIsGrowing` false)))
    (`SceneComponent.SetWorldScale3D` (`self.PlantMesh`) (`KismetMathLibrary.Conv_DoubleToVector` (`KismetMathLibrary.Lerp` (`self.GrowthStartScale`) (+ (`self.BaseFinalScale`) (* (`self.FertilizeCurrent`) (`self.FertilizeGrowthMultiplier`))) (/ (`self.GrowthTimeCurrent`) (`self.GrowthTimeMax`)))))
    ;[1 1 1] Debug UI parameter
    (bind _output_get (set `self.FinalScale` (+ (`self.BaseFinalScale`) (* (`self.FertilizeCurrent`) (`self.FertilizeGrowthMultiplier`)))))
    (if (== (`SceneComponent.K2_GetComponentScale` (`self.PlantMesh`)) (`KismetMathLibrary.Conv_DoubleToVector` _output_get) :`ErrorTolerance` 0.0)
      (`self.Finish Growing Dispatcher`))
    (return)
    (else
      (return))))

(fn `Select`
  (returns (ReturnValue :type Boolean))
  (`KismetSystemLibrary.PrintString` (`KismetStringLibrary.Concat_StrStr` "Plant Selected:" (`KismetSystemLibrary.GetObjectName` (`self.GetOwner` self))))
  (return false))

(fn `UpdateUI`
  (`SceneComponent.K2_SetWorldTransform` (`self.UI Component`) (`KismetMathLibrary.MakeTransform` (+ (`SceneComponent.K2_GetComponentLocation` (`self.PlantMesh`)) (0.0 0.0 100.0)) (`KismetMathLibrary.Conv_VectorToRotator` (* (`SceneComponent.GetForwardVector` (`PlayerCameraManager.TransformComponent` (`GameplayStatics.GetPlayerCameraManager` 0))) -1)) (`KismetMathLibrary.Conv_DoubleToVector` (`self.UI_Scale`))) false false)
  (bind _asplant_ui (cast `/Game/UMG/Plant_UI` (`WidgetComponent.GetUserWidgetObject` (`self.UI Component`)))
    (:`then`
      (`|ExecutionSequence`
        (:`then_0`
          ;[1 1 1] GrowthText
          (`TextBlock.SetText` (`/Game/UMG/Plant_UI.Text_01` _asplant_ui) (`KismetTextLibrary.Conv_StringToText` (`KismetStringLibrary.Concat_StrStr` (`KismetStringLibrary.LeftChop` (`KismetStringLibrary.Concat_StrStr` "Growth Time:" (`KismetStringLibrary.Conv_DoubleToString` (`self.GrowthTimeCurrent`))) 2) (`KismetStringLibrary.Concat_StrStr` "/" (`KismetStringLibrary.Conv_DoubleToString` (`self.GrowthTimeMax`)))))))
        (:`then_1`
          ;[1 1 1] Water Text
          (`TextBlock.SetText` (`/Game/UMG/Plant_UI.Text_02` _asplant_ui) (`KismetTextLibrary.Conv_StringToText` (`KismetStringLibrary.Concat_StrStr` "Water Level:" (`KismetStringLibrary.Conv_DoubleToString` (`self.WaterCurrentLevel`))))))
        (:`then_2`
          ;[1 1 1] Fertilize Text
          (`TextBlock.SetText` (`/Game/UMG/Plant_UI.Text_03` _asplant_ui) (`KismetTextLibrary.Conv_StringToText` (`KismetStringLibrary.Concat_StrStr` "Fertilize Amount:" (`KismetStringLibrary.Conv_IntToString` (`self.FertilizeCurrent`))))))
        (:`then_3`
          ;[1 1 1] Title Text
          (`TextBlock.SetText` (`/Game/UMG/Plant_UI.Title` _asplant_ui) (`KismetTextLibrary.Conv_StringToText` (`KismetSystemLibrary.GetObjectName` (`self.PlantMesh`)))))
        (:`then_4`
          ;[1 1 1] Final Scale Text
          (`TextBlock.SetText` (`/Game/UMG/Plant_UI.Text_04` _asplant_ui) (`KismetTextLibrary.Conv_StringToText` (`KismetStringLibrary.Concat_StrStr` "FinalScale:" (`KismetStringLibrary.Conv_DoubleToString` (`self.FinalScale`))))))
        (:`then_5`
          (return))))
    (:`CastFailed`
      (return))))

(fn `UserConstructionScript`)