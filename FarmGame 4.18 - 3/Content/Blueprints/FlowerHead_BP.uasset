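; Flower head actor that plays its skeletal mesh animation once its parent plant finishes growing.
; On BeginPlay it pauses the animation, hides its static mesh and binds to grow-finished and release dispatchers on its parent Flower_BP or FlowerStem_BP.
; FinishedFlowering fires a done-flowering dispatcher without identifying which head finished.
; The release event is a stub that only prints a debug string.
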(event `self.ReceiveBeginPlay`
  (bind _returnvalue (`self.GetParentActor`))
  (bind _flowerparent (`self.FlowerParent`))
  (bind _stemparent (`self.StemParent`))
  (set `SkeletalMeshComponent.bPauseAnims` true (`self.SkeletalMesh`))
  (`SceneComponent.SetVisibility` (`self.StaticMesh`) false false)
  (bind _asflower_bp (cast `/Game/Blueprints/Flower_BP` _returnvalue)
    (:`then`
      (set `self.FlowerParent` _asflower_bp)
      (add `/Game/Blueprints/Plant_BP.Finish Growing Dispatcher` _flowerparent (delegate `Event Play FlowerHead Anim`))
      (add `/Game/Blueprints/Flower_BP.Event Release Flower Heads Dispatcher` _flowerparent (delegate `Event Release Flower Heads`)))
    (:`CastFailed`
      (bind _asflower_stem_bp (cast `/Game/Blueprints/FlowerStem_BP` _returnvalue))
      (set `self.StemParent` _asflower_stem_bp)
      (add `/Game/Blueprints/FlowerStem_BP.Event Finish Growing Dispatcher ` _stemparent (delegate `Event Play FlowerHead Anim`))
      (add `/Game/Blueprints/FlowerStem_BP.Event Release Flowerhead Dispatcher` _stemparent (delegate `Event Release Flower Heads`)))))

(event `Event Play FlowerHead Anim`
  (set `SkeletalMeshComponent.bPauseAnims` false (`self.SkeletalMesh`)))

(event `Event Release Flower Heads`
  (`KismetSystemLibrary.PrintString` "RELEASE FLOWERHEADS"))

(event `Event Finished Flowering`
  ;[1 0 0.775] Add Param to specify which floerhead is done if needed?
  (`self.DoneFlowering Notify Event Dispatcher`))

(fn `UserConstructionScript`)